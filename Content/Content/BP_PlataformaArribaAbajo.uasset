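; BP_PlataformaArribaAbajo is a moving platform actor, named for vertical up-and-down movement.
; On BeginPlay it stores its initial location and plays a Timeline.
; Each update picks the start-up or start-down track from the EmpiezaMviendoArriba flag and passes it to ChangeActorLocationByTimeLine.
; That function sets the actor's location to the stored origin plus the track offset, without sweeping.
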(event `self.ReceiveBeginPlay`
  (set `self.PosicionInicialPlataforma` (`self.K2_GetActorLocation`))
  (bind (_direction _empiezaarribatrack _empiezaabajotrack) (`Timeline|PlataformaArribaAbajoTimeline`)
    (:`Update`
      (if (`self.EmpiezaMviendoArriba`)
        (`self.ChangeActorLocationByTimeLine` _empiezaarribatrack)
        (else
          (`self.ChangeActorLocationByTimeLine` _empiezaabajotrack))))))

(fn `ChangeActorLocationByTimeLine`
  (params (Track :type "Vector Structure"))
  (`self.K2_SetActorLocation` (+ Track (`self.PosicionInicialPlataforma`))))

(fn `UserConstructionScript`)