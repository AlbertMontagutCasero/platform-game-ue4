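; BP_Enemy is an enemy actor that moves along a timeline-driven path relative to where it starts.
; BeginPlay stores the starting location and plays MovimientoEnemigoTimeline, whose updates feed either the XMov or YMov track, chosen by MovimientoEnX, into ChangeActorLocationByTimeLine.
; That function adds the track value to the stored start and sets the location without sweeping.
; The overlap event is empty and Tick is unused.
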(event `self.ReceiveBeginPlay`
  (set `self.PosicionInicial` (`self.K2_GetActorLocation`))
  (bind (_direction _xmov _ymov) (`Timeline|MovimientoEnemigoTimeline`)
    (:`Update`
      (if (`self.MovimientoEnX`)
        (`self.ChangeActorLocationByTimeLine` _xmov)
        (else
          (`self.ChangeActorLocationByTimeLine` _ymov))))))

(fn `ChangeActorLocationByTimeLine`
  (params (Track :type "Vector Structure"))
  (`self.K2_SetActorLocation` (+ Track (`self.PosicionInicial`))))

(fn `UserConstructionScript`)